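; BP_Door is a level-transition door that shows a prompt plane and text while something overlaps its box and tracks that state in IsOverlapped.
; On BeginPlay it shows the keyhole only if Key is set and yaws the plane by Angle.
; OpenLevel loads LevelName directly for unlocked doors.
; Keyed doors load it only if CheckKey matches KeyNeeded, which is currently tested against a hardcoded "None".
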(event OnComponentBeginOverlap(Box)
  (params (OverlappedComponent :type Primitive%20Component%20Object%20Reference) (OtherActor :type Actor%20Object%20Reference) (OtherComp :type Primitive%20Component%20Object%20Reference) (OtherBodyIndex :type Integer) (bFromSweep :type Boolean) (SweepResult :type Hit%20Result%20Structure%20%28by%20ref%29))
  (Rendering|SetVisibility (Variables|Default|GetPlane) true false)
  (Rendering|SetVisibility (Variables|Default|GetTextRender) true false)
  (Variables|Default|Setis_overlapped true))

(event OnComponentEndOverlap(Box)
  (params (OverlappedComponent :type Primitive%20Component%20Object%20Reference) (OtherActor :type Actor%20Object%20Reference) (OtherComp :type Primitive%20Component%20Object%20Reference) (OtherBodyIndex :type Integer))
  (Rendering|SetVisibility (Variables|Default|GetPlane) false false)
  (Rendering|SetVisibility (Variables|Default|GetTextRender) false false)
  (Variables|Default|Setis_overlapped false))

(event EventBeginPlay
  (if (Variables|Default|Getkey)
    (Rendering|SetVisibility (Variables|Default|Getkeyhole) true false)
    (else
      (Rendering|SetVisibility (Variables|Default|Getkeyhole) false false)))
  (Transformation|AddWorldRotation (Variables|Default|GetPlane) (Math|Rotator|MakeRotator 0.0 0.0 (Variables|Default|Getangle)) false false))

(fn ConstructionScript)

(fn CheckKey
  (params (key_name :type Name))
  (return (Utilities|Name|Equal(Name) key_name (Variables|Default|Getkey_needed))))

(fn OpenLevel
  (if (Variables|Default|Getkey)
    (bind _has_key (CallFunction|CheckKey "None"))
    (if _has_key
      (Game|OpenLevel(byName) (Variables|Default|Getlevel_name)))
    (else
      (Game|OpenLevel(byName) (Variables|Default|Getlevel_name)))))