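; Test tube actor whose liquid fill level goes up in steps each time something overlaps its Box trigger.
; BeginPlay applies the configured material to the Liquid component.
; Each overlap applies a transform scale derived from StartScale, increments Filled and has the first Cheese_table actor run CheckIngredients.
; At the scale limit, an overlap zeroes the scale and count without notifying the table; the trailing Delay gates nothing.
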(event OnComponentBeginOverlap(Box)
  (params (OverlappedComponent :type Primitive%20Component%20Object%20Reference) (OtherActor :type Actor%20Object%20Reference) (OtherComp :type Primitive%20Component%20Object%20Reference) (OtherBodyIndex :type Integer) (bFromSweep :type Boolean) (SweepResult :type Hit%20Result%20Structure%20%28by%20ref%29))
  (if (== (Variables|Default|Getstart_scale) 3.5)
    (Class|SceneComponent|AddLocalTransform (Variables|Default|Getliquid) (Math|Transform|MakeTransform "0, 0, 0" "0, 0, 0" (Math|Vector|MakeVector 3.0 1.0 0.0)) false false)
    (Variables|Default|Setstart_scale 0.0)
    (Variables|Default|Setfilled 0)
    (else
      (Class|SceneComponent|AddLocalTransform (Variables|Default|Getliquid) (Math|Transform|MakeTransform "0, 0, 0" "0, 0, 0" (Math|Vector|MakeVector 3.0 1.0 (+ (Variables|Default|Getstart_scale) 0.5))) false false)
      (Variables|Default|Setstart_scale (+ (Variables|Default|Getstart_scale) 0.5))
      (bind _output_get (Variables|Default|Setfilled (+ (Variables|Default|Getfilled) 1)))
      (Development|PrintString (Utilities|String|ToString(Integer) _output_get))
      (bind _outactors (Actor|GetAllActorsOfClass "/Game/Blueprints/cheese_table.cheese_table_C"))
      (Default|CheckIngredients (Utilities|Array|Get(acopy) _outactors))))
  (Utilities|FlowControl|Delay 0.5))

(event EventBeginPlay
  (Rendering|Material|SetMaterial (Variables|Default|Getliquid) 0 (Variables|Default|Getliquid_material_name)))

(event Collision|EventActorBeginOverlap
  (params (OtherActor :type Actor%20Object%20Reference)))

(event EventTick
  (params (DeltaSeconds :type Float%20%28single-precision%29)))

(fn ConstructionScript)