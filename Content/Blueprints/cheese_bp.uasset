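; Player-controlled cheese actor that moves as a physics object by applying impulses to its static mesh.
; Horizontal and Vertical axes push it along world X and Y scaled by Speed, and Jump adds an upward impulse with no ground check.
; Hits play a randomized volume and pitch impact sound, throttled by position-change checks and a DoOnce reset after a random delay.
; Angular impulse nodes are present but never run.
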(event Collision|EventHit
  (params (MyComp :type Primitive%20Component%20Object%20Reference) (Other :type Actor%20Object%20Reference) (OtherComp :type Primitive%20Component%20Object%20Reference) (bSelfMoved :type Boolean) (HitLocation :type Vector :default "0, 0, 0") (HitNormal :type Vector :default "0, 0, 0") (NormalImpulse :type Vector :default "0, 0, 0") (Hit :type Hit%20Result%20Structure%20%28by%20ref%29))
  (bind _returnvalue (Transformation|GetWorldLocation MyComp))
  (if (not (Math|Vector|Equal(Vector) _returnvalue (Variables|Default|Getlastworld_location) 0.0001))
    (Variables|Default|Setlastworld_location _returnvalue)
    (if (not (Math|Vector|Equal(Vector) HitLocation (Variables|Default|Getlast_location) 1e+01))
      (Utilities|FlowControl|Sequence
        (:then_0
          (Variables|Default|Setlast_location HitLocation)
          (Utilities|FlowControl|DoOnce false :!label _label
            (:Completed
              (Audio|PlaySoundatLocation "/Game/music/hit_eraser.hit_eraser" HitLocation "0, 0, 0" (Math|Random|RandomFloatinRange 0.1 0.5) (Math|Random|RandomFloatinRange 0.6 0.8) 0.0 0 0 0))))
        (:then_1
          (Utilities|FlowControl|Delay (Math|Random|RandomFloatinRange 0.4 0.7))
          (goto _label Reset))))))

(event Collision|EventActorBeginOverlap
  (params (OtherActor :type Actor%20Object%20Reference)))

(event Input|ActionEvents|InputActionJump
  (params (Key :type Key%20Structure :default "None"))
  (:Pressed
    (Physics|AddImpulse (Variables|Default|GetStaticMesh) (Math|Vector|MakeVector 0.0 0.0 2e+05) "None" false)))

(event Input|AxisEvents|InputAxisHorizontal
  (params (AxisValue :type Float%20%28single-precision%29))
  (Physics|AddImpulse (Variables|Default|GetStaticMesh) (* (Math|Vector|MakeVector AxisValue 0.0 0.0) (Variables|Default|Getspeed)) "None" false))

(event Input|AxisEvents|InputAxisVertical
  (params (AxisValue :type Float%20%28single-precision%29))
  (Physics|AddImpulse (Variables|Default|GetStaticMesh) (* (Math|Vector|MakeVector 0.0 AxisValue 0.0) (Variables|Default|Getspeed)) "None" false))

(fn ConstructionScript)