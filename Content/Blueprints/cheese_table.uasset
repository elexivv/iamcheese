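; Cheese table actor that produces a cheese pickup when the test tubes hold a correct ingredient recipe.
; CheckIngredients finds the first TestTube tagged milk, water and red and compares their Filled levels against two accepted combinations.
; On a match it spawns Pickup_cheese just above the table; nothing in this Blueprint calls the check, and its event graph is empty.
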(event EventBeginPlay)

(event Collision|EventActorBeginOverlap
  (params (OtherActor :type Actor%20Object%20Reference)))

(event EventTick
  (params (DeltaSeconds :type Float%20%28single-precision%29)))

(fn ConstructionScript)

(fn CheckIngredients
  (bind _returnvalue (Transformation|GetActorLocation))
  (bind _returnvalue_2 (Transformation|GetActorLocation))
  (bind (_x _y _z) (Math|Vector|BreakVector _returnvalue))
  (bind (_x_2 _y_2 _z_2) (Math|Vector|BreakVector _returnvalue_2))
  (bind _outactors (Actor|GetAllActorsOfClasswithTag "/Game/Blueprints/TestTube.TestTube_C" "milk"))
  (bind _outactors_2 (Actor|GetAllActorsOfClasswithTag "/Game/Blueprints/TestTube.TestTube_C" "water"))
  (bind _outactors_3 (Actor|GetAllActorsOfClasswithTag "/Game/Blueprints/TestTube.TestTube_C" "red"))
  (if (Math|Boolean|ANDBoolean (== (Variables|/Game/Blueprints/TestTube.TestTube_C|Getfilled (Utilities|Array|Get(acopy) _outactors)) 4) (== (Variables|/Game/Blueprints/TestTube.TestTube_C|Getfilled (Utilities|Array|Get(acopy) _outactors_2)) 6) (== (Variables|/Game/Blueprints/TestTube.TestTube_C|Getfilled (Utilities|Array|Get(acopy) _outactors_3)) 1))
    (Game|SpawnActorfromClass "/Game/Blueprints/pickup_cheese.pickup_cheese_C" (Math|Transform|MakeTransform (Math|Vector|MakeVector _x _y (+ _z 5e+01)) "0, 0, 0" "1,1,1") "AlwaysSpawn" 0 0)
    (elif (Math|Boolean|ANDBoolean (== (Variables|/Game/Blueprints/TestTube.TestTube_C|Getfilled (Utilities|Array|Get(acopy) _outactors)) 3) (== (Variables|/Game/Blueprints/TestTube.TestTube_C|Getfilled (Utilities|Array|Get(acopy) _outactors_2)) 2) (== (Variables|/Game/Blueprints/TestTube.TestTube_C|Getfilled (Utilities|Array|Get(acopy) _outactors_3)) 6))
      (Game|SpawnActorfromClass "/Game/Blueprints/pickup_cheese.pickup_cheese_C" (Math|Transform|MakeTransform (Math|Vector|MakeVector _x_2 _y_2 (+ _z_2 5e+01)) "0, 0, 0" "1,1,1") "AlwaysSpawn" 0 0))))