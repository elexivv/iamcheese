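; Mouse vent actor that shows a visual prompt while something overlaps its Box trigger.
; Begin and end overlap toggle the visibility of a Plane and a TextRender, without propagating to children, and set the IsOverlapped flag to match.
; The overlapping actor is not filtered, and nothing in this Blueprint reads the flag.
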(event OnComponentBeginOverlap(box)
  (params (OverlappedComponent :type Primitive%20Component%20Object%20Reference) (OtherActor :type Actor%20Object%20Reference) (OtherComp :type Primitive%20Component%20Object%20Reference) (OtherBodyIndex :type Integer) (bFromSweep :type Boolean) (SweepResult :type Hit%20Result%20Structure%20%28by%20ref%29))
  (Rendering|SetVisibility (Variables|Default|GetPlane) true false)
  (Rendering|SetVisibility (Variables|Default|GetTextRender) true false)
  (Variables|Default|Setis_overlapped true))

(event OnComponentEndOverlap(box)
  (params (OverlappedComponent :type Primitive%20Component%20Object%20Reference) (OtherActor :type Actor%20Object%20Reference) (OtherComp :type Primitive%20Component%20Object%20Reference) (OtherBodyIndex :type Integer))
  (Rendering|SetVisibility (Variables|Default|GetPlane) false false)
  (Rendering|SetVisibility (Variables|Default|GetTextRender) false false)
  (Variables|Default|Setis_overlapped false))

(fn ConstructionScript)