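; Readable note actor that shows story text in the HUD_Cheese dialogue widget while cheese_bp overlaps its box.
; BeginPlay fills the Text array from the Diary1 or Notebook flag; the Diary2 branch is empty.
; Entering the box shows MouseWidget with the first line; leaving hides it and resets the player's TextIndex.
; DisplayText shows the line at a given index, wrapping to the first and returning true when one past the end.
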(event OnComponentBeginOverlap(box)
  (params (OverlappedComponent :type Primitive%20Component%20Object%20Reference) (OtherActor :type Actor%20Object%20Reference) (OtherComp :type Primitive%20Component%20Object%20Reference) (OtherBodyIndex :type Integer) (bFromSweep :type Boolean) (SweepResult :type Hit%20Result%20Structure%20%28by%20ref%29))
  (Utilities|Casting|CastTocheese_bp OtherActor)
  (Variables|Default|Setis_overlapping true)
  (bind _outactors (Actor|GetAllActorsOfClass "/Game/HUD/HUD_Cheese.HUD_Cheese_C"))
  (Widget|SetVisibility (Variables|/Game/HUD/HUD_Cheese.HUD_Cheese_C|GetMouse_Widget (Utilities|Array|Get(acopy) _outactors)) "Visible")
  (Variables|Default|SetNewVar_0 (Variables|/Game/HUD/mousenpc_widget.mousenpc_widget_C|GetDialogue_Text (Variables|/Game/HUD/HUD_Cheese.HUD_Cheese_C|GetMouse_Widget (Utilities|Array|Get(acopy) _outactors))))
  (CallFunction|DisplayText))

(event OnComponentEndOverlap(box)
  (params (OverlappedComponent :type Primitive%20Component%20Object%20Reference) (OtherActor :type Actor%20Object%20Reference) (OtherComp :type Primitive%20Component%20Object%20Reference) (OtherBodyIndex :type Integer))
  (bind _ascheese_bp (Utilities|Casting|CastTocheese_bp OtherActor))
  (Variables|/Game/Blueprints/cheese_bp.cheese_bp_C|Settext_index _ascheese_bp 0)
  (Variables|Default|Setis_overlapping false)
  (bind _outactors (Actor|GetAllActorsOfClass "/Game/HUD/HUD_Cheese.HUD_Cheese_C"))
  (Widget|SetVisibility (Variables|/Game/HUD/HUD_Cheese.HUD_Cheese_C|GetMouse_Widget (Utilities|Array|Get(acopy) _outactors)) "Hidden"))

(event EventBeginPlay
  (if (Variables|Default|GetDiary1)
    (Variables|Default|Settext (Utilities|Array|MakeArray "If you're reading this, we are running out of time. You don't know me but you soon will. For now, remember march, eyes, half of months. 
- Moz"))
    (elif (Variables|Default|GetNotebook)
      (Variables|Default|Settext (Utilities|Array|MakeArray "Wer are getting closer every day to discovering the truth." "Soon  it will be within our grasp."))
      (elif (Variables|Default|GetDiary2)
        _))))

(event Collision|EventActorBeginOverlap
  (params (OtherActor :type Actor%20Object%20Reference)))

(event EventTick
  (params (DeltaSeconds :type Float%20%28single-precision%29)))

(fn ConstructionScript)

(fn DisplayText
  (params (index :type Integer))
  (bind _newvar_0 (Variables|Default|GetNewVar_0))
  (bind _text (Variables|Default|Gettext))
  (if (== index (+ (Utilities|Array|LastIndex _text) 1))
    (Rendering|Components|TextRender|SetText _newvar_0 (Utilities|Array|Get(acopy) _text))
    (Variables|Default|Setindex 0)
    (return true)
    (else
      (Rendering|Components|TextRender|SetText _newvar_0 (Utilities|Array|Get(acopy) _text index))
      (return false))))