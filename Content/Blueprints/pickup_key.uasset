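; Key pickup actor that the cheese_bp actor collects by colliding with it, using a Hit event rather than an overlap.
; Its KeyType selects which key flag to set on GameInstanceCheese (Level3, Level4 or End), so the key persists across level loads.
; The actor destroys itself once a flag is set, and an unrecognized KeyType leaves it in place.
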(event EventBeginPlay
  (|CallParentFunction) ; This node is disabled and will not be called.\nDrag off pins to build functionality.
)

(event Collision|EventActorBeginOverlap
  (params (OtherActor :type Actor%20Object%20Reference)))

(event EventTick
  (params (DeltaSeconds :type Float%20%28single-precision%29))
  (|CallParentFunction DeltaSeconds) ; This node is disabled and will not be called.\nDrag off pins to build functionality.
)

(event Collision|EventHit
  (params (MyComp :type Primitive%20Component%20Object%20Reference) (Other :type Actor%20Object%20Reference) (OtherComp :type Primitive%20Component%20Object%20Reference) (bSelfMoved :type Boolean) (HitLocation :type Vector :default "0, 0, 0") (HitNormal :type Vector :default "0, 0, 0") (NormalImpulse :type Vector :default "0, 0, 0") (Hit :type Hit%20Result%20Structure%20%28by%20ref%29))
  (Utilities|Casting|CastTocheese_bp Other)
  (bind _asgame_instance_cheese (Utilities|Casting|CastToGameInstanceCheese (Game|GetGameInstance)))
  (if (Utilities|Name|Equal(Name) (Variables|Default|Getkey_type) "Level3")
    (Variables|/Game/GameModes/GameInstanceCheese.GameInstanceCheese_C|Sethas_key_level3 _asgame_instance_cheese true)
    (Actor|DestroyActor)
    (elif (Utilities|Name|Equal(Name) (Variables|Default|Getkey_type) "Level4")
      (Variables|/Game/GameModes/GameInstanceCheese.GameInstanceCheese_C|Sethas_key_level4 _asgame_instance_cheese true)
      (Actor|DestroyActor)
      (elif (Utilities|Name|Equal(Name) (Variables|Default|Getkey_type) "End")
        (Variables|/Game/GameModes/GameInstanceCheese.GameInstanceCheese_C|Sethas_key_end _asgame_instance_cheese true)
        (Actor|DestroyActor)))))

(fn ConstructionScript
  (|CallParentFunction))