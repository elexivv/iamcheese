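; Reactive platform for an ordered-step puzzle, identified by its PlatformNum.
; On box overlap it skips repeat hits on the same platform via LastHitPlatform in GameInstanceCheese, then finds the first unset entry in the shared PlatformArray.
; A matching index sets that entry and calls CheckBoxOpened, while a mismatch clears the array to restart the sequence.
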(event OnComponentBeginOverlap(box)
  (params (OverlappedComponent :type Primitive%20Component%20Object%20Reference) (OtherActor :type Actor%20Object%20Reference) (OtherComp :type Primitive%20Component%20Object%20Reference) (OtherBodyIndex :type Integer) (bFromSweep :type Boolean) (SweepResult :type Hit%20Result%20Structure%20%28by%20ref%29))
  (bind _platform_num (Variables|Default|Getplatform_num))
  (bind _platform_num_2 (Variables|Default|Getplatform_num))
  (bind _asgame_instance_cheese (Utilities|Casting|CastToGameInstanceCheese (Game|GetGameInstance)))
  (if (not (== (Variables|/Game/GameModes/GameInstanceCheese.GameInstanceCheese_C|Getlast_hit_platform _asgame_instance_cheese) _platform_num_2))
    (Variables|/Game/GameModes/GameInstanceCheese.GameInstanceCheese_C|Setlast_hit_platform _asgame_instance_cheese _platform_num_2)
    (bind (_array_element _array_index) (Utilities|Array|ForEachLoopwithBreak (Variables|/Game/GameModes/GameInstanceCheese.GameInstanceCheese_C|Getplatform_array _asgame_instance_cheese) :!label _label)
      (:LoopBody
        (if (not _array_element)
          (if (== _array_index _platform_num)
            (Default|SetArrIndex _asgame_instance_cheese _platform_num true)
            (Default|CheckBoxOpened _asgame_instance_cheese)
            (goto _label Break)
            (else
              (for (_ _array_index_2) (Variables|/Game/GameModes/GameInstanceCheese.GameInstanceCheese_C|Getplatform_array _asgame_instance_cheese)
                (Default|SetArrIndex _asgame_instance_cheese _array_index_2 false))
              (goto _label Break))))))))

(event EventBeginPlay)

(event Collision|EventActorBeginOverlap
  (params (OtherActor :type Actor%20Object%20Reference)))

(event EventTick
  (params (DeltaSeconds :type Float%20%28single-precision%29)))

(fn ConstructionScript)