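; Cheese Blueprint that the player moves around by applying physics impulses to its StaticMesh component.
; Horizontal and Vertical axis inputs push it along world X and Y, scaled by Speed, with no delta-time scaling.
; Jump applies a fixed upward impulse with no grounded check.
; Two angular impulse nodes are left unconnected and never run.
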(event Input|ActionEvents|InputActionJump
  (params (Key :type Key%20Structure :default "None"))
  (:Pressed
    (Physics|AddImpulse (Variables|Default|GetStaticMesh) (Math|Vector|MakeVector 0.0 0.0 2e+05) "None" false)))

(event Input|AxisEvents|InputAxisHorizontal
  (params (AxisValue :type Float%20%28single-precision%29))
  (Physics|AddImpulse (Variables|Default|GetStaticMesh) (* (Math|Vector|MakeVector AxisValue 0.0 0.0) (Variables|Default|Getspeed)) "None" false))

(event Input|AxisEvents|InputAxisVertical
  (params (AxisValue :type Float%20%28single-precision%29))
  (Physics|AddImpulse (Variables|Default|GetStaticMesh) (* (Math|Vector|MakeVector 0.0 AxisValue 0.0) (Variables|Default|Getspeed)) "None" false))

(fn ConstructionScript)